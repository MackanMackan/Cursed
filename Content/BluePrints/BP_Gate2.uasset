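; BP_Gate2 is a padlocked double gate that opens when a BP_Key1 actor overlaps the padlock collider.
; The key's physics and collision are disabled, it snaps to the KeyInput point, and a timeline turns it while padlock audio plays.
; After a three-second delay the padlock and key are destroyed, then OpenGates plays sounds and swings both gates through timelines rotating Arrow components as pivots.
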(event OnComponentBeginOverlap(PadLockCollider)
  (params (OverlappedComponent :type Primitive%20Component%20Object%20Reference) (OtherActor :type Actor%20Object%20Reference) (OtherComp :type Primitive%20Component%20Object%20Reference) (OtherBodyIndex :type Integer) (bFromSweep :type Boolean) (SweepResult :type Hit%20Result%20Structure%20%28by%20ref%29))
  (bind _keyinput (Variables|Default|GetKeyInput))
  (bind _relativerotation (Variables|/Script/Engine.SceneComponent|GetRelativeRotation _keyinput))
  (bind _asbp_key_1 (Utilities|Casting|CastToBP_Key1 OtherActor))
  (Physics|SetSimulatePhysics (Variables|/Game/BluePrints/BP_Key1.BP_Key1_C|GetKey _asbp_key_1) false)
  (Collision|SetCollisionEnabled (Variables|/Game/BluePrints/BP_Key1.BP_Key1_C|GetKey _asbp_key_1) "NoCollision")
  (Transformation|SetWorldLocation (Variables|/Game/BluePrints/BP_Key1.BP_Key1_C|GetKey _asbp_key_1) (Transformation|GetWorldLocation _keyinput) false false)
  (Audio|Components|Audio|Play (Variables|Default|GetPadlockAudio) 0.0)
  (bind _turn (Timeline|TurnKeyTimeline Play)
    (:Update
      (Transformation|SetWorldRotation (Variables|/Game/BluePrints/BP_Key1.BP_Key1_C|GetKey _asbp_key_1) (Math|Rotator|MakeRotator (.roll _relativerotation) _turn (.yaw _relativerotation)) false false)
      (Utilities|FlowControl|Delay 3.0)
      (Components|DestroyComponent (Variables|Default|Get21932_Pad_Lock_v1_NEW))
      (Actor|DestroyActor _asbp_key_1)
      (CallFunction|OpenGates))))

(event Custom|OpenGates
  (Audio|PlaySoundatLocation "/Game/SFX/LeftGateOpening.LeftGateOpening" (Transformation|GetWorldLocation (Variables|Default|GetArrow1)) "0, 0, 0" 1.0 1.0 0.0 0 0 0 0)
  (Audio|PlaySoundatLocation "/Game/SFX/RightGateOpening.RightGateOpening" (Transformation|GetWorldLocation (Variables|Default|GetArrow)) "0, 0, 0" 1.0 1.0 0.0 0 0 0 0)
  (bind _turngate (Timeline|OpenLeftGate Play)
    (:Update
      (Transformation|SetRelativeRotation (Variables|Default|GetArrow1) (Math|Rotator|MakeRotator 0.0 0.0 _turngate) false false)
      (bind _turngate_2 (Timeline|OpenRightGate Play)
        (:Update
          (Transformation|SetRelativeRotation (Variables|Default|GetArrow) (Math|Rotator|MakeRotator 0.0 0.0 _turngate_2) false false))))))

(event EventBeginPlay)

(event Collision|EventActorBeginOverlap
  (params (OtherActor :type Actor%20Object%20Reference)))

(event EventTick
  (params (DeltaSeconds :type Float%20%28single-precision%29)))

(fn ConstructionScript)