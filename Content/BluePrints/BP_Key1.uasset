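; BP_Key1 is a key pickup that the player carries in hand and can throw.
; On overlap with an empty-handed player, it attaches to the camera, disables physics and collision, and updates the held-item label.
; ThrowStone detaches it, restores physics and applies force toward a component trace hit or along camera forward, plus upward force.
; Key impacts spawn spark effects, throttled by a short delay.
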(event OnComponentHit(Key)
  (params (HitComponent :type Primitive%20Component%20Object%20Reference) (OtherActor :type Actor%20Object%20Reference) (OtherComp :type Primitive%20Component%20Object%20Reference) (NormalImpulse :type Vector :default "0, 0, 0") (Hit :type Hit%20Result%20Structure%20%28by%20ref%29))
  (if (Variables|Default|GetCanEmit)
    (Niagara|SpawnSystematLocation "/Game/PatricleSystems/PS_Spark.PS_Spark" (Transformation|GetWorldLocation (Variables|Default|GetKey)))
    (Variables|Default|SetCanEmit false)
    (Utilities|FlowControl|Delay 0.33)
    (Variables|Default|SetCanEmit true)))

(event Custom|ThrowStone
  (bind _bp_player (Variables|Default|GetBP_Player))
  (bind _key (Variables|Default|GetKey))
  (bind _key_2 (Variables|Default|GetKey))
  (bind _returnvalue (Transformation|GetWorldLocation _key_2))
  (bind _camera (Variables|/Game/BluePrints/BP_Player.BP_Player_C|GetCamera _bp_player))
  ;[0.1621 0.09329 1] Throw Stone
  (Transformation|DetachFromActor "KeepWorld" "KeepWorld" "KeepRelative")
  (Physics|SetSimulatePhysics _key true)
  (Collision|SetCollisionEnabled _key "PhysicsOnly")
  (Collision|SetCollisionEnabled (Variables|Default|GetStoneCollider) "QueryOnly")
  (bind (_hitlocation _hitnormal _bonename _outhit _returnvalue_2) (Collision|LineTraceComponent _key_2 _returnvalue (+ _returnvalue (* (Math|Vector|GetForwardVector _camera) (Variables|Default|GetLineTranceLength))) true false false))
  (if _returnvalue_2
    (Physics|AddForce _key (+ (* (Math|Vector|GetForwardVector (Math|Rotator|FindLookatRotation _returnvalue _hitlocation)) (Variables|Default|GetForcePower)) (* (Math|Vector|GetUpVector _camera) (Variables|Default|GetForcePowerUp))) "None" false)
    (else
      (Physics|AddForce _key (+ (* (Math|Vector|GetForwardVector _camera) (Variables|Default|GetForcePower)) (* (Math|Vector|GetUpVector _camera) (Variables|Default|GetForcePowerUp))) "None" false)))
  (Rendering|Components|TextRender|SetText (Variables|/Game/UI/W_Crosshair.W_Crosshair_C|GetHoldingInHand (Variables|/Game/BluePrints/BP_Player.BP_Player_C|GetCrosshair (Variables|Default|GetBP_Player))) ""))

(event EventBeginPlay
  (bind _returnvalue (Actor|GetActorOfClass "/Game/BluePrints/BP_Player.BP_Player_C"))
  (Variables|Default|SetBP_Player _returnvalue))

(event Collision|EventActorBeginOverlap
  (params (OtherActor :type Actor%20Object%20Reference))
  (bind _key (Variables|Default|GetKey))
  (bind _bp_player (Variables|Default|GetBP_Player))
  ;[1 0.1895 0.1995] Pick Up Key
  (Utilities|FlowControl|Sequence
    (:then_0
      (bind _asbp_player (Utilities|Casting|CastToBP_Player OtherActor))
      (if (not (Variables|/Game/BluePrints/BP_Player.BP_Player_C|GetHoldingStone _asbp_player))
        (Transformation|SetActorLocation (+ (Transformation|GetWorldLocation (Variables|/Game/BluePrints/BP_Player.BP_Player_C|GetCamera _asbp_player)) (* (Math|Vector|GetForwardVector (Variables|/Game/BluePrints/BP_Player.BP_Player_C|GetCamera _asbp_player)) (Variables|Default|GetStoneLengthForward)) (* (Math|Vector|GetRightVector (Variables|/Game/BluePrints/BP_Player.BP_Player_C|GetCamera _asbp_player)) (Variables|Default|GetStoneLengthRight)) (* (Math|Vector|GetUpVector (Variables|/Game/BluePrints/BP_Player.BP_Player_C|GetCamera _asbp_player)) (Variables|Default|GetStoneLengthLeft))) false false)
        (Transformation|AttachComponentToComponent (Variables|/Game/BluePrints/BP_Player.BP_Player_C|GetCamera _asbp_player) "None" "KeepWorld" "KeepRelative" "KeepRelative" true)
        (Variables|/Game/BluePrints/BP_Player.BP_Player_C|SetHoldingStone _asbp_player true)
        (Physics|SetSimulatePhysics _key false)
        (Collision|SetCollisionEnabled _key "NoCollision")
        (Collision|SetCollisionEnabled (Variables|Default|GetStoneCollider) "NoCollision")
        (Variables|/Game/BluePrints/BP_Player.BP_Player_C|SetKeyInHand _bp_player self)
        (Rendering|Components|TextRender|SetText (Variables|/Game/UI/W_Crosshair.W_Crosshair_C|GetHoldingInHand (Variables|/Game/BluePrints/BP_Player.BP_Player_C|GetCrosshair _bp_player)) "Key")
        (Transformation|SetActorRelativeScale3D "10.000000,10.000000,10.000000")
        (Transformation|SetRelativeRotation (Variables|Default|GetKey) "0, 0, 0" false false)))))

(fn ConstructionScript)