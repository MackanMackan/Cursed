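; Player character that walks, jumps, throws held stones, keys or a hammer, and takes damage from zombies.
; Axis inputs drive movement, controller yaw and clamped spring-arm pitch, while a velocity-gated timeline plays randomized footstep sounds.
; Zombie overlaps lower health shown on the crosshair widget created at BeginPlay, and reload MainLevel when it runs out.
; Holding CallHammer with empty hands recalls the hammer every Tick with a flying sound.
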(event Custom|Take%20Damage
  ;[1 1 1] Take Damage
  (bind _output_get (Variables|Default|SetHealth (- (Variables|Default|GetHealth) 10)))
  (Rendering|Components|TextRender|SetText (Variables|/Game/UI/W_Crosshair.W_Crosshair_C|GetHealth (Variables|Default|GetCrosshair)) (Utilities|Text|ToText(Integer) _output_get))
  (if (<= (Variables|Default|GetHealth) 0)
    (Game|OpenLevel(byName) "MainLevel")))

(event Custom|PlayAmbianceMusic
  (bind _ambiancemusic (Variables|Default|GetAmbianceMusic))
  (Audio|Components|Audio|SetSound _ambiancemusic "/Game/SFX/DarkForestAmbianceAndMusic.DarkForestAmbianceAndMusic")
  (Audio|Components|Audio|Play _ambiancemusic 0.0))

(event Custom|FootStep
  (if (> (Math|Vector|VectorLength (Variables|/Script/Engine.MovementComponent|GetVelocity (Variables|Character|GetCharacterMovement))) 0.1)
    (if (!= (.z (Transformation|GetVelocity)) 0.0)
      (Timeline|FootstepTimeLine Stop
        (:Footstep
          (Audio|PlaySoundatLocation (.OutItem (Utilities|Array|Random (Variables|Default|GetFootSteps))) (Transformation|GetWorldLocation (Variables|Default|GetCamera)) "0, 0, 0" 0.5 (Math|Random|RandomFloatinRange 0.8 1.2) 0.0 0 0 0 0)))
      (else
        (Timeline|FootstepTimeLine Play)))
    (else
      (Timeline|FootstepTimeLine Stop))))

(event Custom|CreateUI
  ;[1 1 1] Create UI
  (bind _returnvalue (UserInterface|CreateWidget "/Game/UI/W_Crosshair.W_Crosshair_C" 0 "Holding"))
  (UserInterface|Viewport|AddtoViewport _returnvalue 0)
  (Variables|Default|SetCrosshair _returnvalue))

(event EventBeginPlay
  (Utilities|FlowControl|Sequence
    (:then_0
      (CallFunction|CreateUI))
    (:then_1
      (CallFunction|PlayAmbianceMusic))
    (:then_2
      (Variables|Default|SetPlayerDialogAudio (Variables|Default|GetMyDialogAudio)))))

(event Collision|EventActorBeginOverlap
  (params (OtherActor :type Actor%20Object%20Reference))
  (Utilities|Casting|CastToBP_ZombieWalk OtherActor)
  (CallFunction|TakeDamage))

(event EventTick
  (params (DeltaSeconds :type Float%20%28single-precision%29))
  (CallFunction|FootStep)
  (if (Variables|Default|GetCallingHammer)
    (Default|CallHammer (Variables|Default|GetHammerRef))))

(event Input|ActionEvents|InputActionJump
  (params (Key :type Key%20Structure :default "None"))
  (:Pressed
    (Character|Jump)))

(event Input|ActionEvents|InputActionThrow
  (params (Key :type Key%20Structure :default "None"))
  (bind _stoneinhand (Variables|Default|GetStoneInHand))
  (bind _hammerinhand (Variables|Default|GetHammerInHand))
  (bind _keyinhand (Variables|Default|GetKeyInHand))
  (:Pressed
    (if (Variables|Default|GetHoldingStone)
      (Utilities|FlowControl|Sequence
        (:then_0
          (Utilities|IsValid _stoneinhand
            (:Is%20Valid
              (Default|ThrowStone _stoneinhand))))
        (:then_1
          (Utilities|IsValid _keyinhand
            (:Is%20Valid
              (Default|ThrowStone _keyinhand))))
        (:then_2
          (Utilities|IsValid _hammerinhand
            (:Is%20Valid
              (Default|Throw _hammerinhand)))))
      (Variables|Default|SetHoldingStone false))))

(event Input|ActionEvents|InputActionCallHammer
  (params (Key :type Key%20Structure :default "None"))
  (bind _hammerref (Variables|Default|GetHammerRef))
  (:Pressed
    (Utilities|IsValid (Variables|Default|GetHammerInHand)
      (:Is%20Not%20Valid
        (if (not (Variables|Default|GetHoldingStone))
          (Utilities|IsValid (Variables|Default|GetHammerRef)
            (:Is%20Valid
              (Variables|Default|SetCallingHammer true)
              (Audio|Components|Audio|Play (Variables|/Game/BluePrints/BP_ThorHammer.BP_ThorHammer_C|GetFlyingSound (Variables|Default|GetHammerRef)) 0.0)))))))
  (:Released
    (Variables|Default|SetCallingHammer false)
    (Utilities|IsValid _hammerref
      (:Is%20Valid
        (Audio|Components|Audio|Stop (Variables|/Game/BluePrints/BP_ThorHammer.BP_ThorHammer_C|GetFlyingSound _hammerref))))))

(event Input|AxisEvents|InputAxisHorizontal
  (params (AxisValue :type Float%20%28single-precision%29))
  ;[1 1 1] Strafe Movement
  (Class|PawnMovementComponent|AddInputVector (Variables|Character|GetCharacterMovement) (* AxisValue (Math|Vector|GetRightVector (Variables|Collision|GetCapsuleComponent))) false))

(event Input|AxisEvents|InputAxisVertical
  (params (AxisValue :type Float%20%28single-precision%29))
  ;[1 1 1] Forward Movement
  (Class|PawnMovementComponent|AddInputVector (Variables|Character|GetCharacterMovement) (* AxisValue (Math|Vector|GetForwardVector (Variables|Collision|GetCapsuleComponent))) false))

(event Input|AxisEvents|InputAxisLookX
  (params (AxisValue :type Float%20%28single-precision%29))
  ;[1 1 1] Look X
  (bind _output_get (Variables|Default|SetLookRotX (+ AxisValue (Variables|Default|GetLookRotX))))
  (Pawn|SetControlRotation (Game|GetPlayerController 0) (Math|Rotator|MakeRotator 0.0 0.0 _output_get)))

(event Input|AxisEvents|InputAxisLookY
  (params (AxisValue :type Float%20%28single-precision%29))
  ;[1 1 1] Look Y
  (bind _output_get (Variables|Default|SetLookRotY (Math|Float|Clamp(Float) (+ AxisValue (Variables|Default|GetLookRotY)) -9e+01 9e+01)))
  (Transformation|SetRelativeRotation (Variables|Default|GetSpringArm) (Math|Rotator|MakeRotator 0.0 _output_get 0.0) false false))

(fn ConstructionScript)