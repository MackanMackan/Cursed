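; BP_PuzzleStructure is a puzzle prop whose crate burns open when a flaming BP_Stone touches it.
; The first stone overlap passes a DoOnce, then, if OnFire, starts fire particles, audio and a timeline-driven light.
; A delay from the timeline update swaps in the open crate mesh, stops the fire and sets BoxDestoryed.
; Tick then plays a second timeline that pitches Arrow1.
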(event Collision|EventActorBeginOverlap
  (params (OtherActor :type Actor%20Object%20Reference))
  (bind _asbp_stone (Utilities|Casting|CastToBP_Stone OtherActor))
  (Utilities|FlowControl|DoOnce false
    (:Completed
      (if (Variables|/Game/BluePrints/BP_Stone.BP_Stone_C|GetOnFire _asbp_stone)
        (Niagara|SetNiagaraVariable(Float) (Variables|Default|GetPS_Fire) "SpawnRate" 5e+01)
        (Audio|Components|Audio|Play (Variables|Default|GetFireAudio) 0.0)
        (bind _firelightintensity (Timeline|Timeline_1 Play)
          (:Update
            (Rendering|Components|Light|SetIntensity (Variables|Default|GetFire) _firelightintensity)
            (Utilities|FlowControl|Delay 5.0)
            (Audio|Components|Audio|Play (Variables|Default|GetDestroyBoxAudio) 0.0)
            (Components|StaticMesh|SetStaticMesh (Variables|Default|GetSM_Crate_Closed) "/Game/AdvancedVillagePack/Meshes/SM_Crate_Open.SM_Crate_Open")
            (Variables|Default|SetBoxDestoryed true)
            (Niagara|SetNiagaraVariable(Float) (Variables|Default|GetPS_Fire) "SpawnRate" 0.0)
            (Audio|Components|Audio|Stop (Variables|Default|GetFireAudio))))))))

(event EventTick
  (params (DeltaSeconds :type Float%20%28single-precision%29))
  (if (Variables|Default|GetBoxDestoryed)
    (bind _newtrack_0 (Timeline|Timeline_0 Play)
      (:Update
        (Transformation|SetRelativeRotation (Variables|Default|GetArrow1) (Math|Rotator|MakeRotator 0.0 _newtrack_0 0.0) false false)))))

(fn ConstructionScript)