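; BP_Stone is a throwable stone that the player picks up by overlap, attaching it to the camera and updating the held-item HUD text.
; ThrowStone restores physics and applies force toward a line-trace hit, or camera forward, plus upward lift.
; Fireplace overlap ignites the stone and destroys it after a delay.
; Hits emit throttled sparks and pitch-randomized sound; overlapping anything except BP_ZombieWalk clears the thrown flag.
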(event OnComponentHit(Stone)
  (params (HitComponent :type Primitive%20Component%20Object%20Reference) (OtherActor :type Actor%20Object%20Reference) (OtherComp :type Primitive%20Component%20Object%20Reference) (NormalImpulse :type Vector :default "0, 0, 0") (Hit :type Hit%20Result%20Structure%20%28by%20ref%29))
  (bind _stone (Variables|Default|GetStone))
  (bind _returnvalue (Transformation|GetWorldLocation _stone))
  ;[1 1 1] Spawn ParticleDust
  (if (Variables|Default|GetCanEmit)
    (Niagara|SpawnSystematLocation "/Game/PatricleSystems/PS_Spark.PS_Spark" _returnvalue)
    (Variables|Default|SetCanEmit false)
    (Audio|PlaySoundatLocation "/Game/SFX/GravelFootstep.GravelFootstep" _returnvalue "0, 0, 0" 1.0 (Math|Random|RandomFloatinRange 0.6 1.8) 0.0 "/Game/SFX/StoneAttenuation.StoneAttenuation" 0 0 0)
    (Utilities|FlowControl|Delay 0.33)
    (Variables|Default|SetCanEmit true)))

(event Custom|ThrowStone
  (bind _bp_player (Variables|Default|GetBP_Player))
  (bind _stone (Variables|Default|GetStone))
  (bind _stone_2 (Variables|Default|GetStone))
  (bind _returnvalue (Transformation|GetWorldLocation _stone_2))
  (bind _camera (Variables|/Game/BluePrints/BP_Player.BP_Player_C|GetCamera _bp_player))
  ;[0.1621 0.09329 1] Throw Stone
  (Transformation|DetachFromActor "KeepWorld" "KeepWorld" "KeepRelative")
  (Physics|SetSimulatePhysics _stone true)
  (Collision|SetCollisionEnabled _stone "QueryAndPhysics")
  (Collision|SetCollisionEnabled (Variables|Default|GetStoneCollider) "QueryOnly")
  (bind (_hitlocation _hitnormal _bonename _outhit _returnvalue_2) (Collision|LineTraceComponent _stone_2 _returnvalue (+ _returnvalue (* (Math|Vector|GetForwardVector _camera) (Variables|Default|GetLineTranceLength))) true false false))
  (if _returnvalue_2
    (Physics|AddForce _stone (+ (* (Math|Vector|GetForwardVector (Math|Rotator|FindLookatRotation _returnvalue _hitlocation)) (Variables|Default|GetForcePower)) (* (Math|Vector|GetUpVector _camera) (Variables|Default|GetForcePowerUp))) "None" false)
    (else
      (Physics|AddForce _stone (+ (* (Math|Vector|GetForwardVector _camera) (Variables|Default|GetForcePower)) (* (Math|Vector|GetUpVector _camera) (Variables|Default|GetForcePowerUp))) "None" false)))
  (Rendering|Components|TextRender|SetText (Variables|/Game/UI/W_Crosshair.W_Crosshair_C|GetHoldingInHand (Variables|/Game/BluePrints/BP_Player.BP_Player_C|GetCrosshair (Variables|Default|GetBP_Player))) "")
  (Variables|Default|SetisThrown true))

(event EventBeginPlay
  (bind _returnvalue (Actor|GetActorOfClass "/Game/BluePrints/BP_Player.BP_Player_C"))
  (Variables|Default|SetBP_Player _returnvalue))

(event Collision|EventActorBeginOverlap
  (params (OtherActor :type Actor%20Object%20Reference))
  (bind _stone (Variables|Default|GetStone))
  (bind _bp_player (Variables|Default|GetBP_Player))
  (bind _bp_player_2 (Variables|Default|GetBP_Player))
  ;[1 0.1895 0.1995] Pick Up Stone
  (Utilities|FlowControl|Sequence
    (:then_0
      (bind _asbp_player (Utilities|Casting|CastToBP_Player OtherActor))
      (if (not (Variables|/Game/BluePrints/BP_Player.BP_Player_C|GetHoldingStone _asbp_player))
        (Transformation|SetActorLocation (+ (Transformation|GetWorldLocation (Variables|/Game/BluePrints/BP_Player.BP_Player_C|GetCamera _asbp_player)) (* (Math|Vector|GetForwardVector (Variables|/Game/BluePrints/BP_Player.BP_Player_C|GetCamera _asbp_player)) (Variables|Default|GetStoneLengthForward)) (* (Math|Vector|GetRightVector (Variables|/Game/BluePrints/BP_Player.BP_Player_C|GetCamera _asbp_player)) (Variables|Default|GetStoneLengthRight)) (* (Math|Vector|GetUpVector (Variables|/Game/BluePrints/BP_Player.BP_Player_C|GetCamera _asbp_player)) (Variables|Default|GetStoneLengthLeft))) false false)
        (Transformation|AttachComponentToComponent (Variables|/Game/BluePrints/BP_Player.BP_Player_C|GetCamera _asbp_player) "None" "KeepWorld" "KeepRelative" "KeepRelative" true)
        (Variables|/Game/BluePrints/BP_Player.BP_Player_C|SetHoldingStone _asbp_player true)
        (Physics|SetSimulatePhysics _stone false)
        (Collision|SetCollisionEnabled _stone "NoCollision")
        (Collision|SetCollisionEnabled (Variables|Default|GetStoneCollider) "NoCollision")
        (Variables|/Game/BluePrints/BP_Player.BP_Player_C|SetStoneInHand _bp_player_2 self)
        (Rendering|Components|TextRender|SetText (Variables|/Game/UI/W_Crosshair.W_Crosshair_C|GetHoldingInHand (Variables|/Game/BluePrints/BP_Player.BP_Player_C|GetCrosshair _bp_player_2)) "Stone")))
    (:then_1
      (Utilities|Casting|CastToBP_Fireplace OtherActor)
      (Utilities|IsValid "/Game/BluePrints/BP_Fireplace.BP_Fireplace"
        (:Is%20Valid
          (Niagara|SetNiagaraVariable(Float) (Variables|Default|GetPS_Fire) "SpawnRate" 5e+01)
          (Variables|Default|SetOnFire true)
          (Utilities|FlowControl|Delay 1e+01)
          (if (Variables|/Game/BluePrints/BP_Player.BP_Player_C|GetHoldingStone _bp_player)
            (if (== self (Variables|/Game/BluePrints/BP_Player.BP_Player_C|GetStoneInHand _bp_player))
              (Variables|/Game/BluePrints/BP_Player.BP_Player_C|SetHoldingStone _bp_player false)
              (Actor|DestroyActor :!label _label)
              (Rendering|Components|TextRender|SetText (Variables|/Game/UI/W_Crosshair.W_Crosshair_C|GetHoldingInHand (Variables|/Game/BluePrints/BP_Player.BP_Player_C|GetCrosshair (Variables|Default|GetBP_Player))) ""))
            (else
              (goto _label))))))
    (:then_2
      (Utilities|Casting|CastToBP_ZombieWalk OtherActor
        (:CastFailed
          (Variables|Default|SetisThrown false))))))

(fn ConstructionScript)