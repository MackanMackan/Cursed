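; BP_Subtitle is a one-shot trigger that plays a sequence of voiced, subtitled dialog lines when BP_Player overlaps it.
; The first overlap disables the box collision and calls PlayDialog, which sets the player's crosshair-widget subtitle and plays the matching clip on the player's audio component.
; PlayDialog re-calls itself after each clip's duration, stepping through parallel text and audio arrays.
; After the last line, a timeline drives the subtitle's opacity fade.
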(event Custom|PlayDialog
  (bind _player (Variables|Default|GetPlayer))
  (bind _player_2 (Variables|Default|GetPlayer))
  (bind _playerdialogaudio (Variables|/Game/BluePrints/BP_Player.BP_Player_C|GetPlayerDialogAudio _player))
  (bind _crosshair (Variables|/Game/BluePrints/BP_Player.BP_Player_C|GetCrosshair _player_2))
  (bind _subtitle (Variables|/Game/UI/W_Crosshair.W_Crosshair_C|GetSubtitle _crosshair))
  (Class|TextBlock|SetOpacity _subtitle 1.0)
  (Rendering|Components|TextRender|SetText _subtitle (Utilities|Array|Get(acopy) (Variables|Default|GetSubtitleText) (Variables|Default|GetLoopAt)))
  (Audio|Components|Audio|SetSound _playerdialogaudio (Utilities|Array|Get(acopy) (Variables|Default|GetDialogAudio) (Variables|Default|GetLoopAt)))
  (Audio|Components|Audio|Play _playerdialogaudio 0.0)
  (Variables|Default|SetLoopAt (+ (Variables|Default|GetLoopAt) 1))
  (Utilities|FlowControl|Delay (Variables|/Script/Engine.SoundBase|GetDuration (Variables|/Script/Engine.AudioComponent|GetSound _playerdialogaudio)))
  (if (< (Variables|Default|GetLoopAt) (Variables|Default|GetLoops))
    (CallFunction|PlayDialog)
    (else
      (bind _fade (Timeline|OpacityFade Play)
        (:Update
          (Class|TextBlock|SetOpacity _subtitle _fade))))))

(event EventBeginPlay)

(event Collision|EventActorBeginOverlap
  (params (OtherActor :type Actor%20Object%20Reference))
  (bind _asbp_player (Utilities|Casting|CastToBP_Player OtherActor))
  (Variables|Default|SetPlayer _asbp_player)
  (Variables|Default|SetLoops (Utilities|Array|Length (Variables|Default|GetSubtitleText)))
  (Utilities|FlowControl|DoOnce false
    (:Completed
      (Collision|SetCollisionEnabled (Variables|Default|GetBox) "NoCollision")
      (CallFunction|PlayDialog))))

(event EventTick
  (params (DeltaSeconds :type Float%20%28single-precision%29)))

(fn ConstructionScript)