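; BP_ThorHammer is a throwable Thor hammer that the player picks up on overlap and can call back.
; Pickup attaches it to the camera with physics off and updates the player's held state and HUD text.
; Throw detaches it and applies force toward a component trace hit or camera forward, while CallHammer pulls it toward the player's camera.
; Zombie overlaps play randomized hit sounds, and physics hits emit rate-limited sparks.
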(event OnComponentHit(Box)
  (params (HitComponent :type Primitive%20Component%20Object%20Reference) (OtherActor :type Actor%20Object%20Reference) (OtherComp :type Primitive%20Component%20Object%20Reference) (NormalImpulse :type Vector :default "0, 0, 0") (Hit :type Hit%20Result%20Structure%20%28by%20ref%29))
  ;[1 1 1] ParticleONGroundHit
  (if (Variables|Default|GetCanEmit)
    (Niagara|SpawnSystematLocation "/Game/PatricleSystems/PS_Spark.PS_Spark" (Transformation|GetWorldLocation (Variables|Default|GetBox)))
    (Variables|Default|SetCanEmit false)
    (Utilities|FlowControl|Delay 0.33)
    (Variables|Default|SetCanEmit true)))

(event Custom|Throw
  (bind _self self)
  (bind _box (Variables|Default|GetBox))
  (bind _box_2 (Variables|Default|GetBox))
  (bind _player (Variables|Default|GetPlayer))
  (bind _martillo_de_thor (Variables|Default|GetMartillo_de_Thor))
  (bind _returnvalue (Transformation|GetWorldLocation _martillo_de_thor))
  (bind _arrow (Variables|Default|GetArrow _self))
  (bind _camera (Variables|/Game/BluePrints/BP_Player.BP_Player_C|GetCamera _player))
  (bind _returnvalue_2 (Transformation|GetWorldRotation _arrow))
  ;[0.9722 1 0.09498] ThrowHammer
  (Transformation|DetachFromActor "KeepWorld" "KeepWorld" "KeepRelative")
  (Variables|/Game/BluePrints/BP_Player.BP_Player_C|SetHammerInHand (Variables|Default|GetPlayer) 0)
  (Collision|SetCollisionEnabled _box "PhysicsOnly")
  (Physics|SetSimulatePhysics _box true)
  (Collision|SetCollisionEnabled (Variables|Default|GetHammerHitCollider) "QueryOnly")
  (bind (_hitlocation _hitnormal _bonename _outhit _returnvalue_3) (Collision|LineTraceComponent _martillo_de_thor _returnvalue (+ _returnvalue (* (Math|Vector|GetForwardVector _camera) (Variables|Default|GetLineTranceLength))) true false false))
  (if _returnvalue_3
    (Physics|AddForce _box_2 (+ (* (Math|Vector|GetForwardVector (Math|Rotator|FindLookatRotation _returnvalue _hitlocation)) (Variables|Default|GetForcePower)) (* (Math|Vector|GetUpVector _camera) (Variables|Default|GetForcePowerUp))) "None" false)
    (else
      (Physics|AddForce _box_2 (+ (* (Math|Vector|GetForwardVector _camera) (Variables|Default|GetForcePower)) (* (Math|Vector|GetUpVector _camera) (Variables|Default|GetForcePowerUp))) "None" false)))
  (Rendering|Components|TextRender|SetText (Variables|/Game/UI/W_Crosshair.W_Crosshair_C|GetHoldingInHand (Variables|/Game/BluePrints/BP_Player.BP_Player_C|GetCrosshair (Variables|Default|GetPlayer))) "")
  (bind _output_get (Variables|Default|SetHammerYRotate (.roll _returnvalue_2)))
  (Transformation|SetWorldRotation _arrow (Math|Rotator|MakeRotator (+ _output_get -76.0) (.pitch _returnvalue_2) (.yaw _returnvalue_2)) false false))

(event Custom|CallHammer
  ;[1 1 1] Calling Hammer
  (Physics|AddForce (Variables|Default|GetBox) (* (Math|Vector|Normalize (- (Transformation|GetWorldLocation (Variables|/Game/BluePrints/BP_Player.BP_Player_C|GetCamera (Variables|Default|GetPlayer))) (Transformation|GetWorldLocation (Variables|Default|GetMartillo_de_Thor)))) (Variables|Default|GetPullForce)) "None" false))

(event EventBeginPlay
  (bind _returnvalue (Actor|GetActorOfClass "/Game/BluePrints/BP_Player.BP_Player_C"))
  (Variables|Default|SetPlayer _returnvalue))

(event EventTick
  (params (DeltaSeconds :type Float%20%28single-precision%29)))

(event Collision|EventActorBeginOverlap
  (params (OtherActor :type Actor%20Object%20Reference))
  (bind _hitsoundsaudio (Variables|Default|GetHitSoundsAudio))
  (bind _player (Variables|Default|GetPlayer))
  (bind _box (Variables|Default|GetBox))
  (bind _box_2 (Variables|Default|GetBox))
  (bind _relativelocation (Variables|/Script/Engine.SceneComponent|GetRelativeLocation _box))
  ;[1 0.1895 0.1995] Pick Up Hammer
  (Utilities|FlowControl|Sequence
    (:then_0
      (bind _asbp_player (Utilities|Casting|CastToBP_Player OtherActor))
      (if (not (Variables|/Game/BluePrints/BP_Player.BP_Player_C|GetHoldingStone _asbp_player))
        (Transformation|SetActorLocation (+ (Transformation|GetWorldLocation (Variables|/Game/BluePrints/BP_Player.BP_Player_C|GetCamera _asbp_player)) (* (Math|Vector|GetForwardVector (Variables|/Game/BluePrints/BP_Player.BP_Player_C|GetCamera _asbp_player)) (Variables|Default|GetStoneLengthForward)) (* (Math|Vector|GetRightVector (Variables|/Game/BluePrints/BP_Player.BP_Player_C|GetCamera _asbp_player)) (Variables|Default|GetStone%20Length%20Right)) (* (Math|Vector|GetUpVector (Variables|/Game/BluePrints/BP_Player.BP_Player_C|GetCamera _asbp_player)) (Variables|Default|GetStone%20Length%20Left))) false false)
        (Transformation|AttachComponentToComponent (Variables|/Game/BluePrints/BP_Player.BP_Player_C|GetCamera _asbp_player) "None" "KeepWorld" "KeepRelative" "KeepRelative" true)
        (Variables|/Game/BluePrints/BP_Player.BP_Player_C|SetHoldingStone _asbp_player true)
        (Physics|SetSimulatePhysics _box_2 false)
        (Collision|SetCollisionEnabled _box_2 "NoCollision")
        (Variables|/Game/BluePrints/BP_Player.BP_Player_C|SetHammerInHand _player self)
        (Rendering|Components|TextRender|SetText (Variables|/Game/UI/W_Crosshair.W_Crosshair_C|GetHoldingInHand (Variables|/Game/BluePrints/BP_Player.BP_Player_C|GetCrosshair _player)) "Thor Hammer")
        (Transformation|SetRelativeLocation _box (Math|Vector|MakeVector (.x _relativelocation) (.y _relativelocation) (+ (.z _relativelocation) 1e+01)) false false)
        (Transformation|SetRelativeRotation (Variables|Default|GetBox) "0,90.000000, 0" false false)
        (Transformation|SetRelativeRotation (Variables|Default|GetArrow) "0, 0, 0" false false)))
    (:then_1
      (Utilities|Casting|CastToBP_ZombieWalk OtherActor)
      (Audio|Components|Audio|SetSound (Variables|Default|GetHitSoundsAudio) (.OutItem (Utilities|Array|Random (Variables|Default|GetHitSounds))))
      (Audio|Components|Audio|SetPitchMultiplier _hitsoundsaudio (Math|Random|RandomFloatinRange 0.8 1.4))
      (Audio|Components|Audio|Play _hitsoundsaudio 0.0))))

(fn ConstructionScript)