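; BP_TreeBigFire is an actor that makes the lighting of a large tree fire flicker.
; On BeginPlay, a Sequence starts six timelines, each driving the intensity of its own point light from a fire intensity track.
; Later Sequence pins pass through DoOnce nodes to trigger Set New Time on each timeline, with random time offsets apparently meant to keep the lights out of sync.
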(event EventBeginPlay
  (Utilities|FlowControl|Sequence
    (:then_0
      (bind _fireintesity (Timeline|FireLightTM Play)
        (:Update
          (Rendering|Components|Light|SetIntensity (Variables|Default|GetPointLight) _fireintesity))))
    (:then_1
      (bind _fireintesity_2 (Timeline|Timeline_0 Play)
        (:Update
          (Rendering|Components|Light|SetIntensity (Variables|Default|GetPointLight1) _fireintesity_2))))
    (:then_2
      (bind _fireintesity_3 (Timeline|Timeline_1 Play)
        (:Update
          (Rendering|Components|Light|SetIntensity (Variables|Default|GetPointLight2) _fireintesity_3))))
    (:then_3
      (bind _fireintesity_4 (Timeline|Timeline_2 Play)
        (:Update
          (Rendering|Components|Light|SetIntensity (Variables|Default|GetPointLight3) _fireintesity_4))))
    (:then_4
      (bind _fireintesity_5 (Timeline|Timeline_3 Play)
        (:Update
          (Rendering|Components|Light|SetIntensity (Variables|Default|GetPointLight4) _fireintesity_5))))
    (:then_5
      (bind _fireintesity_6 (Timeline|Timeline_4 Play)
        (:Update
          (Rendering|Components|Light|SetIntensity (Variables|Default|GetPointLight5) _fireintesity_6))))
    (:then_6
      (Utilities|FlowControl|DoOnce false
        (:Completed
          (Timeline|FireLightTM SetNewTime))))
    (:then_7
      (Utilities|FlowControl|DoOnce false
        (:Completed
          (Timeline|Timeline_0 SetNewTime))))
    (:then_8
      (Utilities|FlowControl|DoOnce false
        (:Completed
          (Timeline|Timeline_1 SetNewTime))))
    (:then_9
      (Utilities|FlowControl|DoOnce false
        (:Completed
          (Timeline|Timeline_2 SetNewTime))))
    (:then_10
      (Utilities|FlowControl|DoOnce false
        (:Completed
          (Timeline|Timeline_3 SetNewTime))))
    (:then_11
      (Utilities|FlowControl|DoOnce false
        (:Completed
          (Timeline|Timeline_4 SetNewTime))))))

(event Collision|EventActorBeginOverlap
  (params (OtherActor :type Actor%20Object%20Reference)))

(fn ConstructionScript)