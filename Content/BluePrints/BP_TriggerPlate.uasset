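; BP_TriggerPlate is a pressure plate that sinks the first time a BP_Player overlaps it.
; An IsPressed flag is set on that overlap and never cleared here, so the plate moves only once.
; The move is a single FInterpTo step on relative Z toward a lower target, so the drop depends on that frame's delta time rather than animating to the target.
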(event EventBeginPlay)

(event Collision|EventActorBeginOverlap
  (params (OtherActor :type Actor%20Object%20Reference))
  (bind _triggerplate (Variables|Default|GetTriggerPlate))
  (bind _relativelocation (Variables|/Script/Engine.SceneComponent|GetRelativeLocation _triggerplate))
  ;[0.381 0.1271 1] Trigger Plate
  (Utilities|Casting|CastToBP_Player OtherActor)
  (if (not (Variables|Default|GetIsPressed))
    (Transformation|SetRelativeLocation _triggerplate (Math|Vector|MakeVector (.x _relativelocation) (.y _relativelocation) (Math|Interpolation|FInterpTo (.z _relativelocation) (- (.z _relativelocation) 4.5e+02) (Utilities|Time|GetWorldDeltaSeconds) 2.0)) false false)
    (Variables|Default|SetIsPressed true)))

(fn ConstructionScript)