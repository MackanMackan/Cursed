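; BP_WinScenario is an actor that handles the win condition of a zombie game once no zombies are left.
; It caches the BP_Player reference on BeginPlay and checks AmountZombieLeft every Tick, with no logic here that changes that count.
; At zero, it reveals the WinText in the player's Crosshair widget, waits through a short Delay, then opens the MainMenu level.
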(event EventBeginPlay
  (bind _returnvalue (Actor|GetActorOfClass "/Game/BluePrints/BP_Player.BP_Player_C"))
  (Variables|Default|SetPlayer _returnvalue))

(event Collision|EventActorBeginOverlap
  (params (OtherActor :type Actor%20Object%20Reference)))

(event EventTick
  (params (DeltaSeconds :type Float%20%28single-precision%29))
  (if (== (Variables|Default|GetAmountZombieLeft) 0)
    (Class|TextBlock|SetOpacity (Variables|/Game/UI/W_Crosshair.W_Crosshair_C|GetWinText (Variables|/Game/BluePrints/BP_Player.BP_Player_C|GetCrosshair (Variables|Default|GetPlayer))) 1.0)
    (Utilities|FlowControl|Delay 5.0)
    (Game|OpenLevel(byName) "MainMenu")))

(fn ConstructionScript)