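; Zombie spawner actor that releases a limited number of BP_ZombieWalk enemies at its own location.
; BeginPlay caches the BP_Player reference so each zombie spawns with its yaw turned toward the player.
; StartSpawnZombie, not triggered within this Blueprint, waits an initial delay, then calls SpawnZombie.
; SpawnZombie re-calls itself after each delayed spawn, decrementing AmountOfSpawns until it reaches zero.
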(event Custom|SpawnZombie
  (bind _self self)
  (bind _defaultsceneroot (Variables|Default|GetDefaultSceneRoot _self))
  (bind _returnvalue (Transformation|GetWorldLocation _defaultsceneroot))
  (if (> (Variables|Default|GetAmountOfSpawns) 0)
    (Utilities|FlowControl|Delay (Variables|Default|GetSpawnDelay))
    (Game|SpawnActorfromClass "/Game/Models/Characters/ZombieEnemy/Walking/BP_ZombieWalk.BP_ZombieWalk_C" (Math|Transform|MakeTransform _returnvalue (Math|Rotator|MakeRotator 0.0 0.0 (.yaw (Math|Rotator|FindLookatRotation _returnvalue (Transformation|GetWorldLocation (Variables|/Script/Engine.Character|GetCapsuleComponent (Variables|Default|GetPlayer)))))) "1.000000,1.000000,1.000000") "Undefined" 0 0)
    (Variables|Default|SetAmountOfSpawns (- (Variables|Default|GetAmountOfSpawns) 1))
    (CallFunction|SpawnZombie)))

(event Custom|StartSpawnZombie
  (Utilities|FlowControl|Delay (Variables|Default|GetStartSpawnDelay))
  (CallFunction|SpawnZombie))

(event EventBeginPlay
  (bind _returnvalue (Actor|GetActorOfClass "/Game/BluePrints/BP_Player.BP_Player_C"))
  (Variables|Default|SetPlayer _returnvalue))

(event Collision|EventActorBeginOverlap
  (params (OtherActor :type Actor%20Object%20Reference)))

(event EventTick
  (params (DeltaSeconds :type Float%20%28single-precision%29)))

(fn ConstructionScript)