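; BP_ZombieWalk is a walking zombie enemy that chases the player and can be killed with thrown stones.
; PawnSensing stores the seen BP_Player, and Tick reissues AIMoveTo toward it every frame, with no logic to clear the target.
; Overlapping a thrown BP_Stone reduces Health; at zero or below, the Walk component switches to physics simulation and capsule collision is disabled.
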(event OnSeePawn(PawnSensing)
  (params (Pawn :type Pawn%20Object%20Reference))
  (bind _asbp_player (Utilities|Casting|CastToBP_Player Pawn))
  (Variables|Default|SetPlayer _asbp_player))

(event EventBeginPlay)

(event Collision|EventActorBeginOverlap
  (params (OtherActor :type Actor%20Object%20Reference))
  (bind _walk (Variables|Default|GetWalk))
  (bind _asbp_stone (Utilities|Casting|CastToBP_Stone OtherActor))
  (Development|PrintString (Utilities|String|ToString(Boolean) (Variables|/Game/BluePrints/BP_Stone.BP_Stone_C|GetisThrown _asbp_stone)))
  (if (Variables|/Game/BluePrints/BP_Stone.BP_Stone_C|GetisThrown _asbp_stone)
    (Variables|Default|SetHealth (- (Variables|Default|GetHealth) 15))
    (if (<= (Variables|Default|GetHealth) 0)
      (Physics|SetSimulatePhysics _walk true)
      (Collision|SetCollisionEnabled _walk "PhysicsOnly")
      (Collision|SetCollisionEnabled (Variables|Collision|GetCapsuleComponent) "NoCollision"))))

(event EventTick
  (params (DeltaSeconds :type Float%20%28single-precision%29))
  (Utilities|IsValid (Variables|Default|GetPlayer)
    (:Is%20Valid
      (AI|AIMoveTo (Variables|Character|GetCharacterMovement) self "0, 0, 0" (Variables|Default|GetPlayer) 5.0 false))))

(fn ConstructionScript)